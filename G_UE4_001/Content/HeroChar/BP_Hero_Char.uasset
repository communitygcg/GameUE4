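; BP_Hero_Char is the player hero Character Blueprint, handling basic movement, look, jump and sprint input.
; Axis inputs move along the capsule's forward and right vectors and add controller pitch and yaw for looking.
; Jump starts and stops with its button, while holding Sprint sets IsSprinting and switches MaxWalkSpeed between WalkSpeed and SprintSpeed, with WalkSpeed applied on BeginPlay.
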(event `self.ReceiveBeginPlay`
  ;[1 1 1] Base_Speed
  (set `CharacterMovementComponent.MaxWalkSpeed` (`self.Walk_Speed`) (`self.CharacterMovement`)))

(event `InputAction|JumpButton`
  (params (Key :type "Key Structure"))
  ;[1 1 1] Jump_BP
  (:`Pressed`
    (`self.Jump`))
  (:`Released`
    (`self.StopJumping`)))

(event `InputAxis|Move_Forward`
  (params (AxisValue :type "Float (single-precision)"))
  ;[1 1 1] Move_Forward
  (`self.AddMovementInput` (`SceneComponent.GetForwardVector` (`self.CapsuleComponent`)) AxisValue))

(event `InputAxis|Move_Right`
  (params (AxisValue :type "Float (single-precision)"))
  ;[1 1 1] Move_Forward
  (`self.AddMovementInput` (`SceneComponent.GetRightVector` (`self.CapsuleComponent`)) AxisValue))

(event `InputAction|Sprint`
  (params (Key :type "Key Structure"))
  (bind _charactermovement (`self.CharacterMovement`))
  ;[1 1 1] Sprint
  (:`Pressed`
    (set `self.isSprinting` true)
    (set `CharacterMovementComponent.MaxWalkSpeed` (`self.Sprint_Speed`) _charactermovement))
  (:`Released`
    (set `self.isSprinting` false)
    (set `CharacterMovementComponent.MaxWalkSpeed` (`self.Walk_Speed`) _charactermovement)))

(event `InputAxis|Look_Up`
  (params (AxisValue :type "Float (single-precision)"))
  ;[1 1 1] Look_BP
  (`self.AddControllerPitchInput` AxisValue))

(event `InputAxis|Look_Turn`
  (params (AxisValue :type "Float (single-precision)"))
  ;[1 1 1] Look_BP
  (`self.AddControllerYawInput` AxisValue))

(fn `UserConstructionScript`)