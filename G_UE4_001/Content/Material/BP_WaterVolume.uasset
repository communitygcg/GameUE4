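; BP_WaterVolume is a resizable water body with a surface plane, a box volume and a scene capture that supplies depth data to the water material.
; The construction script sizes all three from scale and depth variables, with no active event logic.
; DepthCapture renders through a dynamic post-process depth material into a new render target, hiding the actor itself.
; That texture feeds the plane's dynamic water material as DepthTX.
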(fn `UserConstructionScript`
  (locals (NewLocalVar_0 :type "PostProcessVolume Object Reference"))
  (bind _depthtextureres (`self.DepthTextureRes`))
  (bind _returnvalue (* (`self.VolumeDepth`) 50.0))
  (bind _returnvalue_2 (* (`self.VolumeXYScale`) 10.0))
  ;[1 1 1] RelativeLocation
  (`SceneComponent.SetWorldScale3D` (`self.WaterPlane`) (* (1.0 1.0 1.0) (`self.VolumeXYScale`)))
  (`BoxComponent.SetBoxExtent` (`self.WaterVolume`) (`KismetMathLibrary.MakeVector` _returnvalue_2 _returnvalue_2 _returnvalue) true)
  (`SceneComponent.K2_SetRelativeLocation` (`self.WaterVolume`) (`KismetMathLibrary.MakeVector` 0.0 0.0 (* _returnvalue -5.0)) false false)
  (set `SceneCaptureComponent2D.OrthoWidth` (* (`self.VolumeXYScale`) (`self.CaptureRegion`)) (`self.DepthCapture`))
  (bind _returnvalue_3 (`KismetMaterialLibrary.CreateDynamicMaterialInstance` "/Game/Material/MM_Water_Inst.MM_Water_Inst" "None"))
  (set `self.WaterM` _returnvalue_3)
  (`PrimitiveComponent.SetMaterial` (`self.WaterPlane`) 0 (`self.WaterM`))
  (bind _returnvalue_4 (`KismetMaterialLibrary.CreateDynamicMaterialInstance` "/Game/Material/MM_PostP_Inst.MM_PostP_Inst" "None"))
  (set `self.DepthMaterial` _returnvalue_4)
  (`MaterialInstanceDynamic.SetScalarParameterValue` (`self.DepthMaterial`) "DepthChekDistance" (`self.DepthCheker`))
  (bind _structout (setmembers `PostProcessSettings` :`StructRef` (`SceneCaptureComponent2D.PostProcessSettings` (`self.DepthCapture`)) :`WeightedBlendables` (make `WeightedBlendables` (`|MakeArray` (make `WeightedBlendable` 1.0 (`self.DepthMaterial`)) :!type "WeightedBlendable Structure"))))
  (set `SceneCaptureComponent2D.PostProcessSettings` _structout (`self.DepthCapture`))
  (bind _returnvalue_5 (`KismetRenderingLibrary.CreateRenderTarget2D` _depthtextureres _depthtextureres))
  (bind _output_get (set `self.DepthTexture` _returnvalue_5))
  (set `SceneCaptureComponent2D.TextureTarget` _output_get (`self.DepthCapture`))
  (`MaterialInstanceDynamic.SetTextureParameterValue` (`self.WaterM`) "DepthTX" (`self.DepthTexture`))
  (set `SceneCaptureComponent.HiddenActors` (`|MakeArray` self :!type "Actor Object Reference") (`self.DepthCapture`)))