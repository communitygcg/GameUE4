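; BP_Key_Dor_001 is a usable key actor, filed with static doors, that attaches to the hero character when used.
; BeginPlay resets the key's state enum and caches the player's BP_Hero_Char.
; The USEK event snaps the Key001 component to the Key_Socket on the hero's mesh and advances the enum to its second state.
; The CallD function is an empty stub.
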(event `self.ReceiveBeginPlay`
  (`|ExecutionSequence`
    (:`then_0`
      (set `self.enumKey_01` "NewEnumerator0"))
    (:`then_1`
      (bind _asbp_hero_char (cast `/Game/HeroChar/BP_Hero_Char` (`GameplayStatics.GetPlayerCharacter` 0)))
      (set `self.Hero_Char` _asbp_hero_char))))

(event `/Game/GameLogic/Usable/Dors/StaticDor/BP_Use_Interface.USE_K`
  (`SceneComponent.K2_AttachToComponent` (`self.Key_001`) (`Character.Mesh` (`self.Hero_Char`)) "Key_Socket" "SnapToTarget" "SnapToTarget" "SnapToTarget" true)
  (set `self.enumKey_01` "NewEnumerator1"))

(fn `Call_D`
  (return))

(fn `UserConstructionScript`)