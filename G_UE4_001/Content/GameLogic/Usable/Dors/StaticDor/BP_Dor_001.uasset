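; BP_Dor_001 is a static door that slides upward when used with its key in the required state.
; BeginPlay caches the hero and casts the door's own Owner to BP_Key_Dor_001 as the key.
; USEK sets a zero-time looping timer, then checks the key's enum before playing a timeline.
; The timeline lerps the first BP_Dor_001 found in the world, not self, from its current location toward FOpenDor above it.
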(event `self.ReceiveBeginPlay`
  (`|ExecutionSequence`
    (:`then_0`
      (bind _asbp_hero_char (cast `/Game/HeroChar/BP_Hero_Char` (`GameplayStatics.GetPlayerCharacter` 0)))
      (set `self.Hero_Char` _asbp_hero_char))
    (:`then_1`
      (bind _asbp_key_dor_001 (cast `/Game/GameLogic/Usable/Dors/StaticDor/BP_Key_Dor_001` (`self.GetOwner`)))
      (set `self.Key` _asbp_key_dor_001))))

(event `/Game/GameLogic/Usable/Dors/StaticDor/BP_Use_Interface.USE_K`
  (`KismetSystemLibrary.K2_SetTimerDelegate` (delegate `/Game/GameLogic/Usable/Dors/StaticDor/BP_Use_Interface.USE_K`) 0.0 true)
  (if (`|EnumEquality` (`/Game/GameLogic/Usable/Dors/StaticDor/BP_Key_Dor_001.enumKey_01` (`self.Key`)) "NewEnumerator1")
    (bind _outactors (`GameplayStatics.GetAllActorsOfClass` "BP_Dor_001_C"))
    (bind (_direction _move_dor) (`Timeline|Timeline`)
      (:`Update`
        (bind _output (`|GetArrayItem` _outactors))
        (bind (_returnvalue_x _returnvalue_y _returnvalue_z) (`KismetMathLibrary.BreakVector` (`self.K2_GetActorLocation` _output)))
        (`self.K2_SetActorLocation` _output (`KismetMathLibrary.VLerp` (`KismetMathLibrary.MakeVector` _returnvalue_x _returnvalue_y _returnvalue_z) (`KismetMathLibrary.MakeVector` _returnvalue_x _returnvalue_y (+ _returnvalue_z (`self.fOpen_Dor`))) _move_dor) false false)))))

(fn `Call_D`
  (return))

(fn `UserConstructionScript`)